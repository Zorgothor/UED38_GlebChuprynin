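; BP_PlayerCharacter is the player character Blueprint, adding noise reporting, presumably for AI hearing, on top of its parent class.
; ActionMain calls the parent, then uses a resettable DoOnce to report a noise and play a gunshot sound once per press.
; A debug key reports the same noise with an alarm sound.
; Movement-based noise, quieter when crouched, exists but is disconnected from Tick and never runs.
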(event EventBeginPlay
  (|CallParentFunction))

(event Collision|EventActorBeginOverlap
  (params (OtherActor :type Actor%20Object%20Reference)))

(event EventTick
  (params (DeltaSeconds :type Float%20%28single-precision%29))
  ;[1 1 1] Sounds While Moving
)

(event Input|KeyboardEvents|DebugKey1
  (params (Key :type Key%20Structure :default "None") (ActionValue :type Input%20Action%20Value%20Structure))
  (:Pressed
    (Class|AISenseHearing|ReportNoiseEvent (Transformation|GetWorldLocation (Variables|Default|GetCapsuleComponent)) 1.0 self 0.0 "Noise")
    (Audio|PlaySound2D "/Game/Retro_8Bit_Sounds/Alarms_Sirens/Cues/retro_alarm_siren_loop_06_Cue.retro_alarm_siren_loop_06_Cue" 1.0 1.0 0.0 0 0)))

(fn ConstructionScript
  (|CallParentFunction))

(fn ActionMain
  (params (IsPressed :type Boolean))
  (|CallParentFunction IsPressed)
  (if (Variables|Default|GetIsActionMainPressed)
    (Utilities|FlowControl|DoOnce false :!label _label
      (:Completed
        (Class|AISenseHearing|ReportNoiseEvent (Transformation|GetWorldLocation (Variables|Default|GetCapsuleComponent)) 1.0 self 0.0 "Noise")
        (Audio|PlaySound2D "/Game/Retro_8Bit_Sounds/Weapons/Cues/retro_weapon_gun_misc_shot_06_Cue.retro_weapon_gun_misc_shot_06_Cue" 1.0 1.0 0.0 0 0)))
    (else
      (goto _label Reset))))