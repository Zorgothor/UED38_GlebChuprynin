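; BP_CharacterBase is a character base Blueprint providing interaction, damage intake and a main-action input state.
; InteractSphere overlaps store an actor implementing BPI_CustomInterface; Use sends it InteractMessage, and any end overlap clears it.
; AnyDamage casts the damage type to BP_DamageObject and forwards amount, type and causer to BPMainStatsComponent, ignoring other damage types.
; ActionMain only records whether the main action is pressed.
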(event `self.InteractSphere.OnComponentBeginOverlap`
  (params (OverlappedComponent :type "PrimitiveComponent Object Reference") (OtherActor :type "Actor Object Reference") (OtherComp :type "PrimitiveComponent Object Reference") (OtherBodyIndex :type Integer) (bFromSweep :type Boolean) (SweepResult :type "HitResult Structure (by ref)"))
  (if (`KismetSystemLibrary.DoesImplementInterface` OtherActor "/Game/Blueprints/BPI_CustomInterface.BPI_CustomInterface_C")
    (set `self.ActorToInteract` OtherActor)))

(event `self.InteractSphere.OnComponentEndOverlap`
  (params (OverlappedComponent :type "PrimitiveComponent Object Reference") (OtherActor :type "Actor Object Reference") (OtherComp :type "PrimitiveComponent Object Reference") (OtherBodyIndex :type Integer))
  (set `self.ActorToInteract` null))

(event `self.ReceiveAnyDamage`
  (params (Damage :type "Float (single-precision)") (DamageType :type "DamageType Object Reference") (InstigatedBy :type "Controller Object Reference") (DamageCauser :type "Actor Object Reference"))
  (bind _asbp_damage_object (cast `/Game/Blueprints/Objects/BP_DamageObject` DamageType))
  (`/Game/Blueprints/Components/BP_MainStatsComponent.ReceiveDamage` (`self.BP_MainStatsComponent`) Damage (`/Game/Blueprints/Objects/BP_DamageObject. DamageType` _asbp_damage_object) DamageCauser))

(fn `ActionMain`
  (params (IsPressed :type Boolean))
  (set `self.IsActionMainPressed` IsPressed))

(fn `Use`
  (bind _actortointeract (`self.ActorToInteract`)
    (:`then`
      (message `/Game/Blueprints/BPI_CustomInterface.Interact` _actortointeract))
    (:`else`)))

(fn `UserConstructionScript`)