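; BP_NPC_Tiny_A is an NPC character Blueprint that shows its AI state on a tooltip facing the player.
; After the parent Tick, LookAtPlayerCamera runs each frame while LookAt is set.
; It reads AIState from the BP_AIController, writes it to ToolTipText, and rotates that text toward the BP_PlayerCharacter camera.
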(event `self.ReceiveTick`
  (params (DeltaSeconds :type "Float (single-precision)"))
  (`parent.ReceiveTick` DeltaSeconds)
  (`self.LookAtPlayerCamera`))

(fn `LookAtPlayerCamera`
  (if (`self.LookAt`)
    (bind _asbp_aicontroller (cast `/Game/Blueprints/Controller/BP_AIController` (`self.GetController`)))
    (bind _asbp_player_character (cast `/Game/Blueprints/Character/Player/BP_PlayerCharacter` (`GameplayStatics.GetPlayerPawn` 0)))
    (set `self.CameraLocation ` (`SceneComponent.K2_GetComponentLocation` (`/Game/Blueprints/Character/Player/BP_PlayerCharacter.Camera` _asbp_player_character)))
    (`TextRenderComponent.K2_SetText` (`self.ToolTipText`) (`|FormatText` "{AIState}" (`|GetEnumeratorNameAsString` (`/Game/Blueprints/Controller/BP_AIController.AIState ` _asbp_aicontroller))))
    (`SceneComponent.K2_SetWorldRotation` (`self.ToolTipText`) (`KismetMathLibrary.FindLookAtRotation` (`SceneComponent.K2_GetComponentLocation` (`self.ToolTipText`)) (`self.CameraLocation `)) false false)))

(fn `UserConstructionScript`
  (`parent.UserConstructionScript`))