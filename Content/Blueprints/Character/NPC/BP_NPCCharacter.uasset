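; NPC character Blueprint, a child class that adds a health bar, death ragdoll and shot sound to inherited behavior.
; BeginPlay hands the character to its W_HealthBar widget to update the displayed HP.
; Tick polls the stats component's IsDead flag and, through a DoOnce, enables mesh collision and physics simulation.
; The ActionMain override calls the parent, then plays a 2D gun sound while the action is pressed.
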(event `self.ReceiveTick`
  (params (DeltaSeconds :type "Float (single-precision)"))
  (if (`/Game/Blueprints/Components/BP_MainStatsComponent.IsDead` (`self.BP_MainStatsComponent`))
    (`/Engine/EditorBlueprintResources/StandardMacros.DoOnce` false
      (:`Completed`
        (`PrimitiveComponent.SetCollisionEnabled` (`self.Mesh`) "QueryAndPhysics")
        (`PrimitiveComponent.SetSimulatePhysics` (`self.Mesh`) true)))))

(event `self.ReceiveBeginPlay`
  (bind _asw_health_bar (cast `/Game/Blueprints/HUD/Widgets/W_HealthBar` (`WidgetComponent.GetUserWidgetObject` (`self.Widget`))))
  (`/Game/Blueprints/HUD/Widgets/W_HealthBar.UpdateCurrentCharacterForHP` _asw_health_bar self))

(fn `ActionMain`
  (params (IsPressed :type Boolean))
  (`parent.ActionMain` IsPressed)
  (if (`self.IsActionMainPressed`)
    (`GameplayStatics.PlaySound2D` "/Game/Retro_8Bit_Sounds/Weapons/Cues/retro_weapon_gun_misc_shot_06_Cue.retro_weapon_gun_misc_shot_06_Cue" 1.0 1.0 0.0 null null)))

(fn `UserConstructionScript`
  (`parent.UserConstructionScript`))