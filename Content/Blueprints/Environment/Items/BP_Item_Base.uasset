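; BP_Item_Base is a base actor for pickup items that shows a text prompt while a character overlaps it.
; Overlap events track the character, and Tick turns the prompt toward the third-person character's follow camera.
; Interact passes the character's backpack component to PutInToBackpack, an empty hook here, and returns true on every path.
; AfterUse plays the pickup sound and destroys the actor, but nothing in this file calls it.
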(event `self.ReceiveBeginPlay`
  (`SceneComponent.SetVisibility` (`self.TextRender`) false true))

(event `self.ReceiveActorBeginOverlap`
  (params (OtherActor :type "Actor Object Reference"))
  (bind _ascharacter (cast `Character` OtherActor))
  (set `self.CharacterInBox` _ascharacter)
  (`SceneComponent.SetVisibility` (`self.TextRender`) true true)
  (set `self.IsReadyToInteract` true)
  (set `self.LookAt` true))

(event `self.ReceiveActorEndOverlap`
  (params (OtherActor :type "Actor Object Reference"))
  (cast `Character` OtherActor)
  (set `self.CharacterInBox` null)
  (`SceneComponent.SetVisibility` (`self.TextRender`) false true)
  (set `self.IsReadyToInteract` false)
  (set `self.LookAt` false))

(event `self.ReceiveTick`
  (params (DeltaSeconds :type "Float (single-precision)"))
  (`self.LookAtPlayerCamera`))

(fn `AfterUse`
  (`GameplayStatics.PlaySound2D` "/Engine/VREditor/Sounds/UI/Object_PickUp.Object_PickUp" 1.0 1.0 0.0 null null)
  (`self.K2_DestroyActor`))

(fn `Interact`
  (returns (Success :type Boolean))
  (if (`self.IsReadyToInteract`)
    (bind _characterinbox (`self.CharacterInBox`)
      (:`then`
        (bind _returnvalue (`self.GetComponentByClass` _characterinbox "/Game/Blueprints/Components/BP_BackPackComponent.BP_BackPackComponent_C"))
        (`/Engine/EditorBlueprintResources/StandardMacros.IsValid` _returnvalue
          (:`Is Valid`
            (`self.PutInToBackpack` _returnvalue)
            (return true))
          (:`Is Not Valid`
            (return true))))
      (:`else`
        (return true)))
    (else
      (return true))))

(fn `LookAtPlayerCamera`
  (locals (`CameraLocation ` :type "Vector Structure"))
  (if (`self.LookAt`)
    (bind _characterinbox (`self.CharacterInBox`)
      (:`then`
        (bind _asbp_third_person_character (cast `/Game/ThirdPerson/Blueprints/BP_ThirdPersonCharacter` _characterinbox))
        (set `local.CameraLocation ` (`SceneComponent.K2_GetComponentLocation` (`/Game/ThirdPerson/Blueprints/BP_ThirdPersonCharacter.FollowCamera` _asbp_third_person_character)))
        (`SceneComponent.K2_SetWorldRotation` (`self.TextRender`) (`KismetMathLibrary.FindLookAtRotation` (`SceneComponent.K2_GetComponentLocation` (`self.TextRender`)) (`local.CameraLocation `)) false false))
      (:`else`))))

(fn `PutInToBackpack`
  (params (InBackpack :type "/Game/Blueprints/Components/BP_BackPackComponent Object Reference")))

(fn `UserConstructionScript`)